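; Component that animates its owning ThirdPersonCharacter without state-machine logic, switching between idle, run and jump from bound movement and jump events.
; LaunchAnimation looks up a data table row by name, swaps skeletal mesh and physics asset, then plays the animation directly.
; SingleAnimation loops clips, skipping repeats by tracked number; movement cannot interrupt a jump.
; AnimationsSequence chains queued clips with length-based timers, but its demo call is disconnected.
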(event Custom|Jump%20Event
  (params (Stop :type Boolean))
  (if Stop
    (Utilities|SingleAnimation "BoredStanding" 2)
    (else
      (Utilities|SingleAnimation "JumpFast" 6))))

(event Custom|Move%20Forward%20Event
  (params (Axis%20Value :type Float%20%28single-precision%29))
  (bind _my_character (Variables|Default|GetMy%20Character))
  (bind _velocity (Variables|/Script/Engine.MovementComponent|GetVelocity _my_character))
  (if (!= (Variables|Default|GetCurrent%20Animation) 6)
    (if (== (Math|Vector|VectorLength _velocity) 0.0)
      (Utilities|SingleAnimation "BoredStanding" 2)
      (elif (== (.Z (Math|Vector|BreakVector _velocity)) 0.0)
        (Utilities|SingleAnimation "Run" 13)))))

(event EventBeginPlay
  (bind _asthird_person_character (Utilities|Casting|CastToThirdPersonCharacter (Components|GetOwner)))
  (Variables|Default|SetMy%20Third%20Person _asthird_person_character)
  (Variables|Default|SetMy%20Mesh (Actor|GetComponentbyClass (Components|GetOwner) "/Script/Engine.SkeletalMeshComponent"))
  (Variables|Default|SetMy%20Character (Actor|GetComponentbyClass (Components|GetOwner) "/Script/Engine.CharacterMovementComponent"))
  (Utilities|SingleAnimation "BoredStanding" 2)
  (EventDispatchers|BindEventtoDispatchAxisMoveForward (Variables|Default|GetMy%20Third%20Person) (delegate Custom|Move%20Forward%20Event))
  (EventDispatchers|BindEventtoDispatchActionJump (Variables|Default|GetMy%20Third%20Person) (delegate Custom|Jump%20Event)))

(fn LaunchAnimation
  (params (AnimationName :type Name) (Loop :type Boolean))
  (bind _my_mesh (Variables|Default|GetMy%20Mesh))
  (if true
    (bind _returnvalue (Utilities|GetDataTableRow "/Game/Characters/Animations/AnimationsTable.AnimationsTable" AnimationName)
      (:then
        (LocalVariables|SetSkeletal%20Mesh (.Mesh (Utilities|Struct|BreakAnimationRowStructure _returnvalue)))
        (LocalVariables|SetAnimation (.Animation (Utilities|Struct|BreakAnimationRowStructure _returnvalue)))
        (LocalVariables|SetPhysics (.Physics (Utilities|Struct|BreakAnimationRowStructure _returnvalue)))
        (Class|SkinnedMeshComponent|SetSkeletalMesh (Variables|Default|GetMy%20Mesh) (LocalVariables|GetSkeletal%20Mesh) true)
        (Components|SkinnedMesh|SetPhysicsAsset (Variables|Default|GetMy%20Mesh) (LocalVariables|GetPhysics) false)
        (Components|Animation|SetAnimation _my_mesh (LocalVariables|GetAnimation))
        (Audio|Components|Audio|Play _my_mesh Loop)
        (bind _returnvalue_2 (Animation|GetPlayLength (LocalVariables|GetAnimation)))
        (return _returnvalue_2))
      (:RowNotFound
        (Development|PrintString "Not found")))
    (else
      (return 0.0))))

(event Custom|Continue%20Animating
  (if (!= (Utilities|Array|Length (Variables|Default|GetAnimationsStack)) 0)
    (bind _output_get (Variables|Default|SetNext%20Animation (Utilities|Array|Get(acopy) (Variables|Default|GetAnimationsStack))))
    (Development|PrintString (Utilities|String|ToString(Name) _output_get))
    (Utilities|Array|RemoveIndex (Variables|Default|GetAnimationsStack))
    (bind _delay (CallFunction|LaunchAnimation (Variables|Default|GetNext%20Animation) false))
    (Utilities|Time|SetTimerbyEvent (delegate Custom|Continue%20Animating) _delay)
    (else
      (return))))