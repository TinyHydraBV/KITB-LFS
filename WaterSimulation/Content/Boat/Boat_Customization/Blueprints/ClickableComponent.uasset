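; Actor component for boat customization that lets the owning actor be picked up and placed on surfaces with the mouse.
; Hovering toggles custom depth on the owner's static mesh, and clicking toggles the carried state.
; While carried, the detached owner follows a per-tick cursor line trace, aligning to the hit normal with a debug sphere drawn.
; A second click attaches it to the last hit actor, keeping world transform.
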(event Custom|OnMouseClicked
  (params (TouchedActor :type Actor%20Object%20Reference) (ButtonPressed :type Key%20Structure :default "None"))
  ;[1 1 1] Bind Events On Mouse Clicked
  (Utilities|IsValid (Variables|Default|GetStaticMeshReference)
    (:Is%20Valid
      (bind _output_get (Variables|Default|SetIsClicked (not (Variables|Default|GetIsClicked))))
      (if _output_get
        (Development|PrintString "Clicked")
        (Transformation|DetachFromActor (Components|GetOwner) "KeepWorld" "KeepWorld" "KeepWorld")
        (else
          (Development|PrintString "NotClicked")
          (bind _surfaceactor (Variables|Default|GetSurfaceActor)
            (:then
              (Transformation|AttachActorToActor (Components|GetOwner) _surfaceactor "None" "KeepWorld" "KeepWorld" "KeepWorld" true))
            (:else)))))))

(event Custom|OnMouseHover
  (params (TouchedActor :type Actor%20Object%20Reference))
  ;[1 1 1] Bind Events On Mouse Hover Start and End
  (Rendering|SetRenderCustomDepth (Variables|Default|GetStaticMeshReference) true))

(event Custom|OnMouseHoverEnd
  (params (TouchedActor :type Actor%20Object%20Reference))
  ;[1 1 1] Bind Events On Mouse Hover Start and End
  (Rendering|SetRenderCustomDepth (Variables|Default|GetStaticMeshReference) false))

(event EventBeginPlay
  (bind _returnvalue (Components|GetOwner))
  (bind _returnvalue_2 (Components|GetOwner))
  (bind _returnvalue_3 (Actor|GetComponentbyClass _returnvalue "/Script/Engine.StaticMeshComponent"))
  ;[1 1 1] Bind Events On Mouse Clicked
  (EventDispatchers|BindEventtoOnClicked _returnvalue (delegate Custom|OnMouseClicked))
  (Utilities|IsValid _returnvalue_3
    (:Is%20Valid
      (Variables|Default|SetStaticMeshReference _returnvalue_3)
      ;[1 1 1] Bind Events On Mouse Hover Start and End
      (EventDispatchers|BindEventtoOnBeginCursorOver _returnvalue_2 (delegate Custom|OnMouseHover))
      (EventDispatchers|BindEventtoOnEndCursorOver _returnvalue_2 (delegate Custom|OnMouseHoverEnd)))))

(event EventTick
  (params (DeltaSeconds :type Float%20%28single-precision%29))
  (bind _returnvalue (Game|GetPlayerController 0))
  (bind _returnvalue_2 (Components|GetOwner))
  (bind (_worldlocation _worlddirection) (Game|Player|ConvertMouseLocationToWorldSpace _returnvalue))
  ;[1 1 1] Make Raycast From Mouse to World and Check If Theres Objects
  (if (Variables|Default|GetIsClicked)
    (bind _outhit (Collision|LineTraceByChannel _worldlocation (+ _worldlocation (* _worlddirection 1e+04)) "TraceTypeQuery1" false 0 "None"))
    (if (.bBlockingHit (Collision|BreakHitResult _outhit))
      (Variables|Default|SetSurfaceActor (.HitActor (Collision|BreakHitResult _outhit)))
      (Transformation|SetActorLocation _returnvalue_2 (.Location (Collision|BreakHitResult _outhit)) false false)
      (Transformation|SetActorRotation _returnvalue_2 (Math|Rotator|MakeRotator (.Roll (Math|Rotator|BreakRotator (Math|Conversions|RotationFromXVector (.Normal (Collision|BreakHitResult _outhit))))) (- (.Pitch (Math|Rotator|BreakRotator (Math|Conversions|RotationFromXVector (.Normal (Collision|BreakHitResult _outhit))))) 9e+01) (.Yaw (Math|Rotator|BreakRotator (Math|Conversions|RotationFromXVector (.Normal (Collision|BreakHitResult _outhit)))))))
      (Rendering|Debug|DrawDebugSphere (.Location (Collision|BreakHitResult _outhit)) 2e+01 12 "(R=1.000000,G=0.000000,B=0.464954,A=1.000000)" 0.0))))