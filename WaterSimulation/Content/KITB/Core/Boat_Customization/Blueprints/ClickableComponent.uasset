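; Actor component for boat customization that lets the player pick up its owning actor with the mouse and place it on surfaces.
; Hovering toggles custom depth on the owner's static mesh, and clicking toggles the carried state.
; While carried, a per-tick cursor line trace snaps the owner to the hit surface, aligned to its normal, or floats it before the camera.
; Clicking again attaches it to the surface actor, if any.
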(event Custom|OnMouseClicked
  (params (TouchedActor :type Actor%20Object%20Reference) (ButtonPressed :type Key%20Structure))
  ;[1 1 1] Bind Events On Mouse Clicked
  (Variables|Default|SetIsClicked (not (Variables|Default|GetIsClicked)))
  (Utilities|IsValid (Variables|Default|GetSurfaceActor)
    (:Is%20Valid
      (if (Variables|Default|GetIsClicked)
        (Development|PrintString "Clicked")
        (Transformation|DetachFromActor (Components|GetOwner) "KeepWorld" "KeepWorld" "KeepWorld")
        (else
          (Development|PrintString "NotClicked")
          (Transformation|AttachActorToActor (Components|GetOwner) (Variables|Default|GetSurfaceActor) "None" "KeepWorld" "KeepWorld" "KeepWorld" true))))))

(event Custom|OnMouseHover
  (params (TouchedActor :type Actor%20Object%20Reference))
  ;[1 1 1] Bind Events On Mouse Hover Start and End
  (Rendering|SetRenderCustomDepth (Variables|Default|GetStaticMeshReference) true))

(event Custom|OnMouseHoverEnd
  (params (TouchedActor :type Actor%20Object%20Reference))
  ;[1 1 1] Bind Events On Mouse Hover Start and End
  (Rendering|SetRenderCustomDepth (Variables|Default|GetStaticMeshReference) false))

(event Custom|SetPlaceable
  (params (CanAttachOnPlace :type Boolean))
  (Variables|Default|SetIsPlaceable CanAttachOnPlace))

(event EventBeginPlay
  (bind _returnvalue (Components|GetOwner))
  (bind _returnvalue_2 (Components|GetOwner))
  (bind _returnvalue_3 (Actor|GetComponentbyClass _returnvalue "/Script/Engine.StaticMeshComponent"))
  ;[1 1 1] Bind Events On Mouse Clicked
  (EventDispatchers|BindEventtoOnClicked _returnvalue (delegate Custom|OnMouseClicked))
  (Utilities|IsValid _returnvalue_3
    (:Is%20Valid
      (Variables|Default|SetStaticMeshReference _returnvalue_3)
      ;[1 1 1] Bind Events On Mouse Hover Start and End
      (EventDispatchers|BindEventtoOnBeginCursorOver _returnvalue_2 (delegate Custom|OnMouseHover))
      (EventDispatchers|BindEventtoOnEndCursorOver _returnvalue_2 (delegate Custom|OnMouseHoverEnd)))))

(event EventTick
  (params (DeltaSeconds :type Float%20%28single-precision%29))
  (bind _returnvalue (Game|GetPlayerController 0))
  (bind _returnvalue_2 (Game|GetPlayerController 0))
  (bind (_worldlocation _worlddirection) (Game|Player|ConvertMouseLocationToWorldSpace _returnvalue))
  (bind (_worldlocation_2 _worlddirection_2) (Game|Player|ConvertMouseLocationToWorldSpace _returnvalue_2))
  ;[1 1 1] Make Raycast From Mouse to World and Check If Theres Objects
  (if (Variables|Default|GetIsClicked)
    (bind _outhit (Collision|LineTraceByChannel _worldlocation_2 (+ _worldlocation_2 (* _worlddirection_2 1e+04)) "TraceTypeQuery3" false 0 "None"))
    (if (.bBlockingHit (Collision|BreakHitResult _outhit))
      ;[1 1 1] Preview object on the surface
      (Variables|Default|SetSurfaceActor (.HitActor (Collision|BreakHitResult _outhit)))
      (Transformation|SetActorLocation (Components|GetOwner) (.Location (Collision|BreakHitResult _outhit)) false false)
      (Transformation|SetActorRotation (Components|GetOwner) (Math|Rotator|MakeRotator (.Roll (Math|Rotator|BreakRotator (Math|Conversions|RotationFromXVector (.Normal (Collision|BreakHitResult _outhit))))) (- (.Pitch (Math|Rotator|BreakRotator (Math|Conversions|RotationFromXVector (.Normal (Collision|BreakHitResult _outhit))))) 9e+01) (.Yaw (Math|Rotator|BreakRotator (Math|Conversions|RotationFromXVector (.Normal (Collision|BreakHitResult _outhit)))))))
      (Rendering|Debug|DrawDebugSphere (.Location (Collision|BreakHitResult _outhit)) 2e+01 12 "(R=1.000000,G=0.000000,B=0.464954,A=1.000000)" 0.0)
      (else
        ;[1 1 1] Just Preview the Object Floating on the screen
        (Variables|Default|SetSurfaceActor 0)
        (Transformation|SetActorLocation (Components|GetOwner) (+ _worldlocation (* _worlddirection 5e+02)) false false)
        (Transformation|SetActorRotation (Components|GetOwner))))))

(fn Callback
  (Development|PrintString "I am called from Clickable Component.")
  (CallFunction|OnMouseClicked (Components|GetOwner)))